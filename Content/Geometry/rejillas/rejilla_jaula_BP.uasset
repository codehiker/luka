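; Cage grate Blueprint that lets the player character, Luka, interact with it to bring up a text widget.
; Box overlap with Luka sets a Near flag and shows an interact prompt widget, which is removed when the overlap ends.
; On BeginPlay it binds to Luka's interact event, which creates the grate's text widget only while Near is set.
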(event OnComponentBeginOverlap(Box)
  (params (OverlappedComponent :type Primitive%20Component%20Object%20Reference) (OtherActor :type Actor%20Object%20Reference) (OtherComp :type Primitive%20Component%20Object%20Reference) (OtherBodyIndex :type Integer) (bFromSweep :type Boolean) (SweepResult :type Hit%20Result%20Structure%20%28by%20ref%29))
  (Utilities|Casting|CastToLuka_BP OtherActor)
  (Variables|Default|Setnear true)
  (bind _returnvalue (UserInterface|CreateWidget "/Game/Interfaz/W_interact.W_interact_C"))
  (UserInterface|Viewport|AddtoViewport _returnvalue 0))

(event OnComponentEndOverlap(Box)
  (params (OverlappedComponent :type Primitive%20Component%20Object%20Reference) (OtherActor :type Actor%20Object%20Reference) (OtherComp :type Primitive%20Component%20Object%20Reference) (OtherBodyIndex :type Integer))
  (Utilities|Casting|CastToLuka_BP OtherActor)
  (Variables|Default|Setnear false)
  (bind _foundwidgets (Widget|GetAllWidgetsOfClass "/Game/Interfaz/W_interact.W_interact_C" true))
  (Widget|RemovefromParent _foundwidgets))

(event Custom|create_widget
  (if (Variables|Default|Getnear)
    (bind _returnvalue (UserInterface|CreateWidget "/Game/Geometry/rejillas/w_rejilla_text_inicio.w_rejilla_text_inicio_C"))
    (UserInterface|Viewport|AddtoViewport _returnvalue 0)))

(event EventBeginPlay
  (bind _asluka_bp (Utilities|Casting|CastToLuka_BP (Game|GetPlayerCharacter 0)))
  (EventDispatchers|BindEventtoLukaInteract _asluka_bp (delegate Custom|create_widget)))

(fn ConstructionScript)