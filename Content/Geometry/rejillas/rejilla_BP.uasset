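; Interactable grate (rejilla) that shows a text widget when the player inspects it up close.
; The Colision component's overlaps with Luka_BP set a Near flag and add or remove an interaction prompt widget.
; Tick polls the first player controller for a right mouse click and, while Near, adds a new text widget to the viewport, with no removal in this Blueprint.
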(event OnComponentBeginOverlap(colision)
  (params (OverlappedComponent :type Primitive%20Component%20Object%20Reference) (OtherActor :type Actor%20Object%20Reference) (OtherComp :type Primitive%20Component%20Object%20Reference) (OtherBodyIndex :type Integer) (bFromSweep :type Boolean) (SweepResult :type Hit%20Result%20Structure%20%28by%20ref%29))
  (Utilities|Casting|CastToLuka_BP OtherActor)
  (Variables|Default|Setnear true)
  (bind _returnvalue (UserInterface|CreateWidget "/Game/Interfaz/W_interact.W_interact_C"))
  (UserInterface|Viewport|AddtoViewport _returnvalue 0))

(event OnComponentEndOverlap(colision)
  (params (OverlappedComponent :type Primitive%20Component%20Object%20Reference) (OtherActor :type Actor%20Object%20Reference) (OtherComp :type Primitive%20Component%20Object%20Reference) (OtherBodyIndex :type Integer))
  (Utilities|Casting|CastToLuka_BP OtherActor)
  (Variables|Default|Setnear false)
  (Widget|RemovefromParent (stale OnComponentBeginOverlap(colision) _returnvalue)))

(event EventBeginPlay)

(event Collision|EventActorBeginOverlap
  (params (OtherActor :type Actor%20Object%20Reference)))

(event EventTick
  (params (DeltaSeconds :type Float%20%28single-precision%29))
  (if (and (Game|Player|WasInputKeyJustPressed (Game|GetPlayerController 0) "RightMouseButton") (Variables|Default|Getnear))
    (bind _returnvalue (UserInterface|CreateWidget "/Game/Geometry/rejillas/w_rejilla_text.w_rejilla_text_C"))
    (UserInterface|Viewport|AddtoViewport _returnvalue 0)))

(fn ConstructionScript)