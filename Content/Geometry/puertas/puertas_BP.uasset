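; Automatic double door Blueprint that opens when the Luka_BP character enters its collision volume and closes when it leaves.
; Overlap begin plays the Open timeline, which lerps the right and left door meshes from their origin to EndDer and EndIzq relative offsets.
; Overlap end reverses the same timeline, and both directions play a 2D door sound.
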(event OnComponentBeginOverlap(collision)
  (params (OverlappedComponent :type Primitive%20Component%20Object%20Reference) (OtherActor :type Actor%20Object%20Reference) (OtherComp :type Primitive%20Component%20Object%20Reference) (OtherBodyIndex :type Integer) (bFromSweep :type Boolean) (SweepResult :type Hit%20Result%20Structure%20%28by%20ref%29))
  (Utilities|Casting|CastToLuka_BP OtherActor)
  (Audio|SpawnSound2D "/Game/sounds/puertas/puerta.puerta" 1.0 1.0 0.0 0)
  (bind _newtrack_0 (Timeline|Open Play)
    (:Update
      (Transformation|SetRelativeLocation (Variables|Default|Getdoor_der) (Math|Vector|Lerp(Vector) "0, 0, 0" (Variables|Default|GetEnd_der) _newtrack_0) false false)
      (Transformation|SetRelativeLocation (Variables|Default|Getdor_izq) (Math|Vector|Lerp(Vector) "0, 0, 0" (Variables|Default|GetEnd_izq) _newtrack_0) false false))))

(event OnComponentEndOverlap(collision)
  (params (OverlappedComponent :type Primitive%20Component%20Object%20Reference) (OtherActor :type Actor%20Object%20Reference) (OtherComp :type Primitive%20Component%20Object%20Reference) (OtherBodyIndex :type Integer))
  (Utilities|Casting|CastToLuka_BP OtherActor)
  (Audio|SpawnSound2D "/Game/sounds/puertas/puerta.puerta" 1.0 1.0 0.0 0)
  (bind _newtrack_0 (Timeline|Open Reverse)
    (:Update
      (Transformation|SetRelativeLocation (Variables|Default|Getdoor_der) (Math|Vector|Lerp(Vector) "0, 0, 0" (Variables|Default|GetEnd_der) _newtrack_0) false false)
      (Transformation|SetRelativeLocation (Variables|Default|Getdor_izq) (Math|Vector|Lerp(Vector) "0, 0, 0" (Variables|Default|GetEnd_izq) _newtrack_0) false false))))

(event EventBeginPlay)

(event Collision|EventActorBeginOverlap
  (params (OtherActor :type Actor%20Object%20Reference)))

(event EventTick
  (params (DeltaSeconds :type Float%20%28single-precision%29)))

(fn ConstructionScript)