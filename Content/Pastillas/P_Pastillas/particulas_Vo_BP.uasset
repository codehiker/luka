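; Particle effect actor for the B_Pastilla_V pill, shown briefly when the Luka_BP character touches it while Volando (flying) is active.
; The particle system starts hidden on BeginPlay.
; On Colision overlap with Luka_BP, it reads Volando from the first B_Pastilla_V found in the level.
; If true, it shows the particles, then hides them after a short delay.
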(event OnComponentBeginOverlap(colision)
  (params (OverlappedComponent :type Primitive%20Component%20Object%20Reference) (OtherActor :type Actor%20Object%20Reference) (OtherComp :type Primitive%20Component%20Object%20Reference) (OtherBodyIndex :type Integer) (bFromSweep :type Boolean) (SweepResult :type Hit%20Result%20Structure%20%28by%20ref%29))
  (Utilities|Casting|CastToLuka_BP OtherActor)
  (bind _outactors (Actor|GetAllActorsOfClass "/Game/Pastillas/B_Pastillas/B_Pastilla_V.B_Pastilla_V_C"))
  (if (Variables|/Game/Pastillas/B_Pastillas/B_Pastilla_V.B_Pastilla_V_C|GetVolando (Utilities|Array|Get(acopy) _outactors))
    (Rendering|SetVisibility (Variables|Default|GetParticleSystem) true false)
    (Utilities|FlowControl|Delay 2.0)
    (Rendering|SetVisibility (Variables|Default|GetParticleSystem) false false)))

(event EventBeginPlay
  (Rendering|SetVisibility (Variables|Default|GetParticleSystem) false false))

(event Collision|EventActorBeginOverlap
  (params (OtherActor :type Actor%20Object%20Reference)))

(fn ConstructionScript)