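; BP_LPunos is a damage-dealing Blueprint, apparently a fist hitbox by its name, that hurts AI characters on contact.
; On overlap it casts the other actor to AICharacter, stores it as Enemigo1 and applies a fixed amount of damage.
; Tick polls only that last stored enemy's Vida, clamping it to zero and destroying the enemy once it is depleted, with no validity check on the reference.
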(event EventBeginPlay)

(event Collision|EventActorBeginOverlap
  (params (OtherActor :type Actor%20Object%20Reference))
  (bind _asaicharacter (Utilities|Casting|CastToAICharacter OtherActor))
  (bind _output_get (Variables|Default|Setenemigo1 _asaicharacter))
  (Game|Damage|ApplyDamage _output_get 1e+02 0 0))

(event EventTick
  (params (DeltaSeconds :type Float%20%28single-precision%29))
  (bind _enemigo1 (Variables|Default|Getenemigo1))
  (if (<= (Variables|/Game/AI/AICharacter.AICharacter_C|Getvida _enemigo1) 0.0)
    (Variables|/Game/AI/AICharacter.AICharacter_C|Setvida _enemigo1 0.0)
    (Actor|DestroyActor (Variables|Default|Getenemigo1))))

(fn ConstructionScript)