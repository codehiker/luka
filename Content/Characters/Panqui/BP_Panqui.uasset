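; BP_Panqui is an interactable character that Luka_BP can talk to.
; A cylinder overlap tracks whether Luka is near, adding the W_interact prompt on entry and removing all top-level instances of it on exit.
; On BeginPlay it binds its talk event to Luka's interact event through the player character, and that event opens the W_panqui widget only while Luka is near.
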(event OnComponentBeginOverlap(Cylinder)
  (params (OverlappedComponent :type Primitive%20Component%20Object%20Reference) (OtherActor :type Actor%20Object%20Reference) (OtherComp :type Primitive%20Component%20Object%20Reference) (OtherBodyIndex :type Integer) (bFromSweep :type Boolean) (SweepResult :type Hit%20Result%20Structure%20%28by%20ref%29))
  (Utilities|Casting|CastToLuka_BP OtherActor)
  (Variables|Default|SetNear true)
  (bind _returnvalue (UserInterface|CreateWidget "/Game/Interfaz/W_interact.W_interact_C"))
  (UserInterface|Viewport|AddtoViewport _returnvalue 0))

(event OnComponentEndOverlap(Cylinder)
  (params (OverlappedComponent :type Primitive%20Component%20Object%20Reference) (OtherActor :type Actor%20Object%20Reference) (OtherComp :type Primitive%20Component%20Object%20Reference) (OtherBodyIndex :type Integer))
  (Utilities|Casting|CastToLuka_BP OtherActor)
  (Variables|Default|SetNear false)
  (bind _foundwidgets (Widget|GetAllWidgetsOfClass "/Game/Interfaz/W_interact.W_interact_C" true))
  (Widget|RemovefromParent _foundwidgets))

(event Custom|talk
  (if (Variables|Default|Getnear)
    (bind _returnvalue (UserInterface|CreateWidget "/Game/Characters/Panqui/w_panqui.w_panqui_C"))
    (UserInterface|Viewport|AddtoViewport _returnvalue 0)))

(event EventBeginPlay
  (bind _asluka_bp (Utilities|Casting|CastToLuka_BP (Game|GetPlayerCharacter 0)))
  (EventDispatchers|BindEventtoLukaInteract _asluka_bp (delegate Custom|talk)))

(event Collision|EventActorBeginOverlap
  (params (OtherActor :type Actor%20Object%20Reference)))

(event EventTick
  (params (DeltaSeconds :type Float%20%28single-precision%29)))

(fn ConstructionScript)